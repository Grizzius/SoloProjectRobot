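; Player character with camera-relative movement, a toggleable sword, HP tracking and a pause menu.
; Movement rounds the Camera1-to-player look-at vectors to whole-number axes, and a Niagara effect runs above a speed threshold.
; Attack plays a DoOnce-gated slash montage that halts movement and locks turning, while StartAttack/EndAttack toggle the hit capsule.
; Capsule overlaps spawn impact effects, drive timeline-based global time dilation and send randomized damage via IsAttackedMessage.
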(event OnComponentBeginOverlap(Capsule)
  (params (OverlappedComponent :type Primitive%20Component%20Object%20Reference) (OtherActor :type Actor%20Object%20Reference) (OtherComp :type Primitive%20Component%20Object%20Reference) (OtherBodyIndex :type Integer) (bFromSweep :type Boolean) (SweepResult :type Hit%20Result%20Structure%20%28by%20ref%29))
  (bind _statattack (Variables|Default|GetStatAttack))
  (Utilities|FlowControl|Sequence
    (:then_0
      (Niagara|SpawnSystematLocation "/Game/Niagara/NGR_AttackImpact.NGR_AttackImpact" (Transformation|GetActorLocation OtherActor))
      (bind _newtrack_0 (Timeline|Timeline_0 PlayFromStart)
        (:Update
          (Utilities|Time|SetGlobalTimeDilation _newtrack_0))))
    (:then_1
      (Class|BPIAttack|IsAttacked(Message) OtherActor (Math|Random|RandomIntegerinRange (- _statattack 5) (+ _statattack 5))))))

(event Custom|StartAttack
  (bind _capsule (Variables|Default|GetCapsule))
  (CallFunction|ToggleSword true)
  (Collision|SetCollisionEnabled _capsule "QueryAndPhysics")
  (Rendering|SetVisibility _capsule true false)
  (Niagara|SpawnSystematLocation "/Game/Niagara/NGR_SwordSlash.NGR_SwordSlash" (Transformation|GetActorLocation) (Transformation|GetActorRotation)))

(event Custom|EndAttack
  (bind _capsule (Variables|Default|GetCapsule))
  (Collision|SetCollisionEnabled _capsule "NoCollision")
  (Rendering|SetVisibility _capsule false false))

(event Custom|ToggleSword
  (params (hasSword :type Boolean))
  (bind _output_get (Variables|Default|SetbHasWeapon hasSword))
  (Rendering|SetVisibility (Variables|Default|GetCapedBotSword) _output_get false))

(event Custom|TakeDamage
  (params (Damage :type Integer))
  (Variables|Default|SetCurrentHP (Math|Integer|Clamp(Integer) (- (Variables|Default|GetCurrentHP) Damage) 0 (Variables|Default|GetMaxHP)))
  (Niagara|SpawnSystematLocation "/Game/Niagara/NGR_AttackImpact.NGR_AttackImpact" (Transformation|GetActorLocation)))

(event EventBeginPlay
  (CallFunction|ToggleSword false))

(event EventTick
  (params (DeltaSeconds :type Float%20%28single-precision%29))
  (Components|Activation|SetActive (Variables|Default|GetNiagara) (> (Math|Vector|VectorLength (Transformation|GetVelocity)) 3e+02) false))

(event Input|ActionEvents|InputActionPauseMenu
  (params (Key :type Key%20Structure :default "None"))
  (:Pressed
    (Variables|/Script/Engine.PlayerController|SetbShowMouseCursor (Game|GetPlayerController 0) true)
    (bind _returnvalue (UserInterface|CreateWidget "/Game/UI/WB_PauseMenu.WB_PauseMenu_C"))
    (UserInterface|Viewport|AddtoViewport _returnvalue 0)
    (Game|SetGamePaused true)))

(event Input|ActionEvents|InputActionGetSword
  (params (Key :type Key%20Structure :default "None"))
  (:Pressed
    (CallFunction|ToggleSword (not (Variables|Default|GetbHasWeapon)))))

(event Input|ActionEvents|InputActionAttack
  (params (Key :type Key%20Structure :default "None"))
  (bind _charactermovement (Variables|Character|GetCharacterMovement))
  (:Pressed
    (Utilities|FlowControl|DoOnce false :!label _label
      (:Completed
        (Utilities|FlowControl|Sequence
          (:then_0
            (Variables|/Script/Engine.CharacterMovementComponent|SetMaxWalkSpeed _charactermovement 0.0)
            (bind _returnvalue (Animation|PlayAnimMontage "/Game/Assets/PlayerCharacter/Animations/CapedBot_Slash_Montage.CapedBot_Slash_Montage" 1.0 "None"))
            (Utilities|FlowControl|Delay (- _returnvalue 0.4))
            (Variables|/Script/Engine.CharacterMovementComponent|SetMaxWalkSpeed _charactermovement 6e+02)
            (Variables|/Script/Engine.CharacterMovementComponent|SetRotationRate (Variables|Character|GetCharacterMovement) "0,1000.000000, 0")
            (Utilities|FlowControl|Delay 0.2)
            (goto _label Reset))
          (:then_1
            (Utilities|FlowControl|Delay 0.1)
            (Variables|/Script/Engine.CharacterMovementComponent|SetRotationRate (Variables|Character|GetCharacterMovement) "0, 0, 0")))))))

(event Input|AxisEvents|InputAxisMoveUp/Down
  (params (AxisValue :type Float%20%28single-precision%29))
  (bind _returnvalue (Transformation|GetActorLocation))
  (bind _camera1 (Variables|Default|GetCamera1))
  (bind _returnvalue_2 (Transformation|GetWorldLocation _camera1))
  (bind _returnvalue_3 (Math|Rotator|FindLookatRotation _returnvalue_2 _returnvalue))
  (bind _returnvalue_4 (Math|Vector|GetForwardVector _returnvalue_3))
  (bind (_x _y _z) (Math|Vector|BreakVector _returnvalue_4))
  (bind _returnvalue_5 (Math|Float|Ceil _x))
  (bind _returnvalue_6 (Math|Float|Ceil _y))
  (bind _returnvalue_7 (Math|Float|Ceil _z))
  (bind _returnvalue_8 (Math|Conversions|ToFloat(Integer) _returnvalue_5))
  (bind _returnvalue_9 (Math|Conversions|ToFloat(Integer) _returnvalue_6))
  (bind _returnvalue_10 (Math|Conversions|ToFloat(Integer) _returnvalue_7))
  (bind _returnvalue_11 (Math|Vector|MakeVector _returnvalue_8 _returnvalue_9 _returnvalue_10))
  (bind (_x_2 _y_2) (Math|Vector|BreakVector _returnvalue_11))
  (Pawn|Input|AddMovementInput (Math|Vector|MakeVector _x_2 _y_2 0.0) AxisValue false))

(event Input|AxisEvents|InputAxisMoveLeft/Right
  (params (AxisValue :type Float%20%28single-precision%29))
  (bind _returnvalue (Transformation|GetActorLocation))
  (bind _camera1 (Variables|Default|GetCamera1))
  (bind _returnvalue_2 (Transformation|GetWorldLocation _camera1))
  (bind _returnvalue_3 (Math|Rotator|FindLookatRotation _returnvalue_2 _returnvalue))
  (bind _returnvalue_4 (Math|Vector|GetRightVector _returnvalue_3))
  (bind (_x _y _z) (Math|Vector|BreakVector _returnvalue_4))
  (bind _return_value (CallFunction|FloororCeil _z))
  (bind _return_value_2 (CallFunction|FloororCeil _x))
  (bind _return_value_3 (CallFunction|FloororCeil _y))
  (bind _returnvalue_5 (Math|Vector|MakeVector _return_value_2 _return_value_3 _return_value))
  (bind (_x_2 _y_2) (Math|Vector|BreakVector _returnvalue_5))
  (Pawn|Input|AddMovementInput (Math|Vector|MakeVector _x_2 _y_2 0.0) AxisValue false))

(fn ConstructionScript)

(fn FloororCeil
  (params (A :type Float%20%28double-precision%29))
  (return (Math|Float|SelectFloat (Math|Conversions|ToFloat(Integer) (Math|Float|Ceil A)) (Math|Conversions|ToFloat(Integer) (Math|Float|Floor A)) (> A 0.0))))