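; Base enemy Blueprint that handles taking damage, showing a health bar and dying.
; IsAttacked forwards damage to TakeDamage, which plays a hit sound, lowers HP unless invincible, and either destroys the actor or updates its WB_HealthBar widget.
; Each call also sets a very brief invincibility window and reveals the hidden health bar, using a timeline's Finished event to hide it again.
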(event Custom|TakeDamage
  (params (DamageAmount :type Integer))
  (bind _widget (Variables|Default|GetWidget))
  (Audio|PlaySoundatLocation "/Game/Audio/SFX_Cue/SFX_MachineDamage.SFX_MachineDamage" (Transformation|GetActorLocation) "0, 0, 0" 1.0 1.0 0.0 0 0 0 0)
  (Utilities|FlowControl|Sequence
    (:then_0
      (if (not (Variables|Default|GetbIsInvincible))
        (bind _output_get (Variables|Default|SetCurrentHP (- (Variables|Default|GetCurrentHP) DamageAmount)))
        (if (<= _output_get 0)
          (CallFunction|Die)
          (else
            (Development|PrintString (Utilities|String|ToString(Integer) _output_get))
            (bind _aswb_health_bar (Utilities|Casting|CastToWB_HealthBar (UserInterface|GetWidget (Variables|Default|GetWidget))))
            (Default|UpdateHealthBar _aswb_health_bar (Variables|Default|GetCurrentHP) (Variables|Default|GetMaxHP))))))
    (:then_1
      (Variables|Default|SetbIsInvincible true)
      (Utilities|FlowControl|Delay 0.05)
      (Variables|Default|SetbIsInvincible false))
    (:then_2
      (Utilities|IsValid _widget
        (:Is%20Valid
          (if (not (Variables|/Script/Engine.SceneComponent|GetbVisible _widget))
            (Rendering|SetVisibility (Variables|Default|GetWidget) true false)
            (Timeline|Timeline_0 PlayFromStart
              (:Finished
                (Rendering|SetVisibility (Variables|Default|GetWidget) false false)))))))))

(event Custom|Die
  (Actor|DestroyActor))

(event EventBeginPlay)

(event Collision|EventActorBeginOverlap
  (params (OtherActor :type Actor%20Object%20Reference)))

(event EventTick
  (params (DeltaSeconds :type Float%20%28single-precision%29)))

(event EventIsAttacked
  (params (RawDamage :type Integer))
  (CallFunction|TakeDamage RawDamage))

(fn ConstructionScript)